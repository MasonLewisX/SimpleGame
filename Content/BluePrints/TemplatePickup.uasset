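; Template pickup item actor that the player can collect into the HUD inventory and later use to raise health, energy and mood.
; A trigger overlap with the character's capsule toggles a widget-component prompt and an in-range flag.
; The character's PickupItem dispatcher adds the item's struct, holding a self-reference, to the inventory and refreshes it.
; The collected actor stays hidden without collision until UseAction applies its stat bonuses and destroys it.
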(event `self.ReceiveBeginPlay`
  (bind _iteminfo (`self.ItemInfo`))
  (bind _pickuptextreference (`self.PickupTextReference`))
  (bind (_item _itemimage _pickuptext) (break `/Game/UMG/InventoryStruct` _iteminfo))
  ;[1 1 1] Event BeginPlay
  ;;[1 1 1] 새로 수정된 부분
  (bind _aspickup_text (cast `/Game/UMG/PickupText` (`WidgetComponent.GetUserWidgetObject` (`self.Widget`))))
  (set `self.PickupTextReference` _aspickup_text)
  (setmembers `/Game/UMG/InventoryStruct` :`StructRef` _iteminfo :`Item` self)
  (set `/Game/UMG/PickupText.PickupActor` _item _pickuptextreference)
  (set `/Game/UMG/PickupText.PickupText` _pickuptext _pickuptextreference)
  (bind _asthird_person_character (cast `/Game/ThirdPersonCPP/Blueprints/ThirdPersonCharacter` (`GameplayStatics.GetPlayerCharacter` 0)))
  (bind _output_get (set `self.Character Reference` _asthird_person_character))
  (add `/Game/ThirdPersonCPP/Blueprints/ThirdPersonCharacter.PickupItem` _output_get (delegate `PickupItem_Event_1`)))

(event `self.ReceiveTick`
  (params (DeltaSeconds :type "Float (single-precision)"))
  ;[1 1 1] Event BeginPlay
)

(event `self.Trigger.OnComponentBeginOverlap`
  (params (OverlappedComponent :type "PrimitiveComponent Object Reference") (OtherActor :type "Actor Object Reference") (OtherComp :type "PrimitiveComponent Object Reference") (OtherBodyIndex :type Integer) (bFromSweep :type Boolean) (SweepResult :type "HitResult Structure (by ref)"))
  ;[1 1 1] Overlap Trigger Script
  (if (== (`GameplayStatics.GetObjectClass` OtherComp) "/Script/Engine.CapsuleComponent")
    (cast `/Game/ThirdPersonCPP/Blueprints/ThirdPersonCharacter` OtherActor)
    (`SceneComponent.SetVisibility` (`self.Widget`) true false)
    (set `self.IsInRange?` true)))

(event `PickupItem_Event_1`
  (bind _game_hud_reference (`/Game/ThirdPersonCPP/Blueprints/ThirdPersonCharacter.Game HUD Reference` (`self.Character Reference`)))
  ;[1 1 1] 아이템을 줍고 인벤토리에 넣은 후 새로고침 하기
  (if (and (`self.IsInRange?`) (`self.GetActorEnableCollision`))
    (`KismetArrayLibrary.Array_Add` (`/Game/UMG/GameHUD.Inventory` _game_hud_reference) (`self.ItemInfo`))
    (`self.SetActorHiddenInGame` true)
    (`self.SetActorEnableCollision` false)
    (`/Game/UMG/GameHUD.RefreshInventory` _game_hud_reference)))

(event `self.Trigger.OnComponentEndOverlap`
  (params (OverlappedComponent :type "PrimitiveComponent Object Reference") (OtherActor :type "Actor Object Reference") (OtherComp :type "PrimitiveComponent Object Reference") (OtherBodyIndex :type Integer))
  ;[1 1 1] Overlap Trigger Script
  (if (== (`GameplayStatics.GetObjectClass` OtherComp) "/Script/Engine.CapsuleComponent")
    (cast `/Game/ThirdPersonCPP/Blueprints/ThirdPersonCharacter` OtherActor)
    (`SceneComponent.SetVisibility` (`self.Widget`) false false)
    (set `self.IsInRange?` false)))

(event `/Game/UMG/ActionInterface.UseAction`
  (bind _character_reference (`self.Character Reference`))
  ;[1 1 1] Use Action
  (set `/Game/ThirdPersonCPP/Blueprints/ThirdPersonCharacter.HealthValue` (+ (`PublicCharacter.Health` _character_reference) (`self.AddHealth`) 0.0) _character_reference)
  (set `/Game/ThirdPersonCPP/Blueprints/ThirdPersonCharacter.EnergyValue` (+ (`/Game/ThirdPersonCPP/Blueprints/ThirdPersonCharacter.EnergyValue` _character_reference) (`self.AddEnergy`)) _character_reference)
  (set `/Game/ThirdPersonCPP/Blueprints/ThirdPersonCharacter.MoodValue` (+ (`/Game/ThirdPersonCPP/Blueprints/ThirdPersonCharacter.MoodValue` _character_reference) (`self.AddMood`)) _character_reference)
  (`self.K2_DestroyActor`))

(fn `UserConstructionScript`)