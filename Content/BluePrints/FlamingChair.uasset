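; Flaming chair projectile that explodes on impact, with randomized damage and critical hits.
; On projectile activation it randomizes InitialSpeed, derives damage from chair mass times speed, and rolls for a critical multiplier.
; Chair hits turn damage into physics impulses, spawn explosion effects, destroy the actor and print the result; projectile stop halts rotation and enables physics.
; Line-trace impact, health subtraction and burning effects are left unconnected, so no health damage is applied.
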(event `self.Chair.OnComponentHit`
  (params (HitComponent :type "PrimitiveComponent Object Reference") (OtherActor :type "Actor Object Reference") (OtherComp :type "PrimitiveComponent Object Reference") (NormalImpulse :type "Vector Structure") (Hit :type "HitResult Structure (by ref)"))
  (bind (_bblockinghit _binitialoverlap _time _distance _location _impactpoint _normal _impactnormal _physmat _hitactor _hitcomponent) (`GameplayStatics.BreakHitResult` Hit))
  (bind (_returnvalue_location _returnvalue_rotation) (`KismetMathLibrary.BreakTransform` (`self.GetTransform` _hitactor)))
  (if (stale `self.ProjectileMovement.OnComponentActivated` _output_get_3)
    (`PrimitiveComponent.AddImpulseAtLocation` _hitcomponent (+ _impactpoint (stale `self.ProjectileMovement.OnComponentActivated` _output_get_4)) (0.0 0.0 0.0) "None") ; 충돌된 지점에 크리티컬 데미지 적용
    (`PrimitiveComponent.AddRadialImpulse` (`self.Chair`) _impactpoint 50.0 0.8 "RIF_Constant" false)
    (`GameplayStatics.SpawnEmitterAtLocation` "/Game/StarterContent/Particles/P_Explosion.P_Explosion" _impactpoint _returnvalue_rotation)
    (`GameplayStatics.PlaySoundAtLocation` "/Game/StarterContent/Audio/Explosion02.Explosion02" _impactpoint (struct) 1.0 1.0 0.0 null null null)
    (`KismetSystemLibrary.Delay` 0.0)
    (`self.K2_DestroyActor`)
    (`KismetSystemLibrary.PrintString` (`KismetStringLibrary.Conv_DoubleToString` (* (stale `self.ProjectileMovement.OnComponentActivated` _output_get_4) 0.01)) true true (struct :`R` 1.0 :`B` 0.019054 :`A` 1.0))
    (`KismetSystemLibrary.PrintString` "치명타!!" true true (struct :`R` 1.0 :`B` 0.019054 :`A` 1.0))
    (else
      (`PrimitiveComponent.AddImpulseAtLocation` _hitcomponent (+ _impactpoint (stale `self.ProjectileMovement.OnComponentActivated` _output_get_5)) (0.0 0.0 0.0) "None")
      (`PrimitiveComponent.AddRadialImpulse` (`self.Chair`) (0.0 0.0 0.0) 50.0 0.8 "RIF_Constant" false)
      (`GameplayStatics.SpawnEmitterAtLocation` "/Game/StarterContent/Particles/P_Explosion.P_Explosion" _impactpoint _returnvalue_rotation)
      (`GameplayStatics.PlaySoundAtLocation` "/Game/StarterContent/Audio/Explosion02.Explosion02" (0.0 0.0 0.0) (struct) 1.0 1.0 0.0 null null null)
      (`KismetSystemLibrary.Delay` 0.0)
      (`self.K2_DestroyActor`)
      (`KismetSystemLibrary.PrintString` (`KismetStringLibrary.Conv_DoubleToString` (* (stale `self.ProjectileMovement.OnComponentActivated` _output_get_5) 0.01)))
      (`KismetSystemLibrary.PrintString` "데미지"))))

(event `self.Box.OnComponentHit`
  (params (HitComponent :type "PrimitiveComponent Object Reference") (OtherActor :type "Actor Object Reference") (OtherComp :type "PrimitiveComponent Object Reference") (NormalImpulse :type "Vector Structure") (Hit :type "HitResult Structure (by ref)")))

(event `self.ProjectileMovement.OnComponentActivated`
  (params (Component :type "ActorComponent Object Reference") (bReset :type Boolean))
  (bind _asprojectile_movement_component (cast `ProjectileMovementComponent` Component))
  (bind _output_get (set `ProjectileMovementComponent.InitialSpeed` (`KismetMathLibrary.RandomFloatInRange` 1000.0 5000.0) _asprojectile_movement_component))
  (`KismetSystemLibrary.PrintString` (`KismetStringLibrary.Conv_DoubleToString` (* _output_get 0.01)) true true (struct :`R` 0.156027 :`G` 0.157986 :`B` 0.153019 :`A` 1.0))
  (`KismetSystemLibrary.PrintString` "던지는 속도 (m/s)" true true (struct :`R` 0.156027 :`G` 0.157986 :`B` 0.153019 :`A` 1.0))
  (bind _output_get_2 (set `self.ChairBaseDamage` (* (`PrimitiveComponent.GetMass` (`self.Chair`)) (* (`ProjectileMovementComponent.InitialSpeed` (`self.ProjectileMovement`)) 1.0))))
  (bind _output_get_3 (set `self.IsItCritical?` (<= (`KismetMathLibrary.RandomFloatInRange` 0.0 100.0) (`self.CriticalHitProbability`))))
  (if _output_get_3
    (bind _output_get_4 (set `self.Damage To Deal` (* _output_get_2 1.8))) ; 치명타 데미지
    (else
      (bind _output_get_5 (set `self.Damage To Deal` _output_get_2)) ; 일반 데미지
    )))

(event `self.ReceiveBeginPlay`)

(event `self.ProjectileMovement.OnProjectileStop`
  (params (ImpactResult :type "HitResult Structure (by ref)"))
  (set `RotatingMovementComponent.RotationRate` (struct) (`self.RotatingMovement`))
  (`PrimitiveComponent.SetSimulatePhysics` (`self.Chair`) true))

(fn `GetPlayerViewPoint`
  (returns (Location :type "Vector Structure") (Rotation :type "Rotator Structure"))
  (locals (MyPlayerController :type "PlayerController Object Reference"))
  (bind _playercameramanager (`PlayerController.PlayerCameraManager` (`local.MyPlayerController`)))
  (bind _output_get (set `local.MyPlayerController` (`GameplayStatics.GetPlayerController` 0)))
  (if (`KismetSystemLibrary.IsValid` _output_get)
    (if (`KismetSystemLibrary.IsValid` _playercameramanager)
      (return (`PlayerCameraManager.GetCameraLocation` _playercameramanager) (`PlayerCameraManager.GetCameraRotation` _playercameramanager)))))

(fn `UserConstructionScript`)