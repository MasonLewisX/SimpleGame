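; Battery pickup Blueprint that plays a particle beam toward the player when collected.
; WasCollected attaches the emitter to the pickup mesh and aims its beam at the player's Spine2 socket.
; A short Delay loop keeps re-aiming the beam, while a longer Delay defers the parent's WasCollected logic.
; An unfinished, unconnected snippet sets the character's EnergyValue, noted as an attempt to fill a UMG mana gauge.
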(event `self.WasCollected`
  (bind _returnvalue (`GameplayStatics.SpawnEmitterAttached` "/Game/Effects/P_explosion_lv1_2.P_explosion_lv1_2" (`self.PickupMesh`) "None" (0.0 0.0 0.0) (struct) (1.0 1.0 1.0) "SnapToTargetIncludingScale"))
  (`ParticleSystemComponent.SetBeamTargetPoint` _returnvalue 0 (`SceneComponent.GetSocketLocation` (`Character.Mesh` (`GameplayStatics.GetPlayerCharacter` 0)) "Spine2") 0 :!label _label)
  (`|ExecutionSequence`
    (:`then_0`
      (`KismetSystemLibrary.Delay` 0.5)
      (`parent.WasCollected`))
    (:`then_1`
      (`KismetSystemLibrary.Delay` 0.1)
      (goto _label))))

(fn `UserConstructionScript`)