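; AI controller for the Steel enemy, running its behavior tree on BeginPlay and on possessing a SteelPlayerCharacter.
; BeginPlay initializes the blackboard with the player character as PlayerKey.
; Perception updates for ThirdPersonCharacter set CanSeePlayer; losing sight sets RecentlySighted and writes the controller's own location to PlayerLocation.
; Walk, run, normal attack and two duplicate jump-attack events forward to the cached possessed pawn.
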(event OnTargetPerceptionUpdated(AIPerception)
  (params (Actor :type Actor%20Object%20Reference) (Stimulus :type AI%20Stimulus%20Structure))
  (bind _bsuccessfullysensed (Utilities|Struct|BreakAIStimulus Stimulus))
  (bind _returnvalue (AI|GetBlackboard 0))
  ;[1 1 1] 플레이어 감지 후 CanSeePlayer bool value true로 지정. 그 후 BehaviorTree 실행 순서에 의해 플레이어쪽으로 이동.
  (Utilities|Casting|CastToThirdPersonCharacter Actor)
  (AI|Components|Blackboard|SetValueasBool _returnvalue (Utilities|Name|MakeLiteralName "CanSeePlayer") _bsuccessfullysensed)
  (if (not _bsuccessfullysensed)
    (AI|Components|Blackboard|SetValueasVector _returnvalue (Utilities|Name|MakeLiteralName "PlayerLocation") (Transformation|GetActorLocation))
    (AI|Components|Blackboard|SetValueasBool _returnvalue (Utilities|Name|MakeLiteralName "RecentlySighted") true)))

(event Custom|Attack_Normal
  (Default|AttackNormal (Variables|Default|GetAISteel)))

(event Custom|Attack_Jump
  (Default|AttackJump (Variables|Default|GetAISteel)))

(event Custom|Walk
  (Default|Walk (Variables|Default|GetAISteel)))

(event Custom|Run
  (Default|Run (Variables|Default|GetAISteel)))

(event Custom|Jump_Attack
  (Default|AttackJump (Variables|Default|GetAISteel)))

(event EventBeginPlay
  (bind _blackboardcomponent (Class|AIController|UseBlackboard "/Game/BluePrints/AI_Steel/EnemyBlackboard_Steel.EnemyBlackboard_Steel"))
  (AI|Components|Blackboard|SetValueasObject _blackboardcomponent (Variables|Default|GetPlayerKey) (Game|GetPlayerCharacter 0))
  (AI|RunBehaviorTree "/Game/BluePrints/AI_Steel/EnemyBehaviorTree_Steel.EnemyBehaviorTree_Steel"))

(event EventTick
  (params (DeltaSeconds :type Float%20%28single-precision%29)))

(event EventPossess
  (params (PossessedPawn :type Pawn%20Object%20Reference))
  (bind _assteel_player_character (Utilities|Casting|CastToSteelPlayerCharacter PossessedPawn))
  (Variables|Default|SetAISteel _assteel_player_character)
  (AI|RunBehaviorTree "/Game/BluePrints/AI_Steel/EnemyBehaviorTree_Steel.EnemyBehaviorTree_Steel"))

(fn ConstructionScript)