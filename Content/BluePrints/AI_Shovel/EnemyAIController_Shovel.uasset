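; AI controller for the shovel enemy that runs its behavior tree on BeginPlay and on possession.
; BeginPlay stores the player character in the shovel blackboard.
; AI perception updates CanSeePlayer and, when sensing fails, records the player's current location and clears RecentlySighted.
; AttackShovel forwards to the possessed AITestCharacter, while Walk, Run and AttackSteel are empty stubs.
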(event `self.ReceiveBeginPlay`
  (bind _blackboardcomponent (`self.UseBlackboard` "/Game/BluePrints/AI_Shovel/EnemyBlackboard_Shovel.EnemyBlackboard_Shovel"))
  (`BlackboardComponent.SetValueAsObject` _blackboardcomponent (`self.PlayerKey`) (`GameplayStatics.GetPlayerCharacter` 0))
  (`self.RunBehaviorTree` "/Game/BluePrints/AI_Shovel/EnemyBehaviorTree_Shovel.EnemyBehaviorTree_Shovel"))

(event `self.AIPerception.OnTargetPerceptionUpdated`
  (params (Actor :type "Actor Object Reference") (Stimulus :type "AIStimulus Structure"))
  (bind (_age _expirationage _strength _stimuluslocation _receiverlocation _tag _bsuccessfullysensed) (break `AIStimulus` Stimulus))
  (bind _returnvalue (`AIBlueprintHelperLibrary.GetBlackboard` null))
  (cast `/Game/ThirdPersonCPP/Blueprints/ThirdPersonCharacter` Actor)
  (`BlackboardComponent.SetValueAsBool` _returnvalue "CanSeePlayer" _bsuccessfullysensed)
  (if (not _bsuccessfullysensed)
    (`BlackboardComponent.SetValueAsVector` _returnvalue "PlayerLocation" (`self.K2_GetActorLocation` (`GameplayStatics.GetPlayerCharacter` 0)))
    (`BlackboardComponent.SetValueAsBool` _returnvalue "RecentlySighted" false)))

(event `Walk`
  ;[1 1 1] 필요없는 부분. 뭘 하던 없어도 됨.
)

(event `Run`
  ;[1 1 1] 필요없는 부분. 뭘 하던 없어도 됨.
)

(event `self.OnPossess`
  (params (PossessedPawn :type "Pawn Object Reference"))
  (bind _asaitest_character (cast `/Game/BluePrints/AI_Shovel/AITestCharacter` PossessedPawn))
  (set `self.AIShovel` _asaitest_character)
  (`self.RunBehaviorTree` "/Game/BluePrints/AI_Shovel/EnemyBehaviorTree_Shovel.EnemyBehaviorTree_Shovel"))

(event `AttackShovel`
  (`/Game/BluePrints/AI_Shovel/AITestCharacter.AttackShovel` (`self.AIShovel`)))

(event `AttackSteel`)

(fn `UserConstructionScript`)