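; Player pawn that moves, jumps, orbits and zooms a spring-arm camera, and fires FlamingChair actors.
; Movement axes offset the location along world X/Y, and a zoom axis adjusts the clamped arm length.
; Holding right mouse opens a Tick gate that rotates the spring arm; releasing snaps the pawn to control rotation.
; Left click spawns a chair ahead along control rotation, offset by fireDirection, whose assignment is never executed.
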(event EventBeginPlay)

(event Collision|EventActorBeginOverlap
  (params (OtherActor :type Actor%20Object%20Reference)))

(event EventTick
  (params (DeltaSeconds :type Float%20%28single-precision%29))
  (Utilities|FlowControl|Gate true
    (:Exit
      (CallFunction|CameraRotation))))

(event Input|AxisEvents|InputAxisCameraZoom
  (params (AxisValue :type Float%20%28single-precision%29))
  (CallFunction|CameraZoom AxisValue))

(event Input|AxisEvents|InputAxisMoveRight
  (params (AxisValue :type Float%20%28single-precision%29))
  (Transformation|SetActorLocationAndRotation (+ (* (Math|Vector|MakeVector 0.0 3.0 0.0) AxisValue) (Transformation|GetActorLocation)) "0, 0, 0"))

(event Input|AxisEvents|InputAxisMoveForward
  (params (AxisValue :type Float%20%28single-precision%29))
  (Transformation|SetActorLocationAndRotation (+ (* (Math|Vector|MakeVector 3.0 0.0 0.0) AxisValue) (Transformation|GetActorLocation)) "0, 0, 0"))

(event Input|KeyboardEvents|SpaceBar
  (params (Key :type Key%20Structure))
  (:Pressed
    (Character|Jump)
    (Transformation|SetActorLocationAndRotation (Transformation|GetActorLocation) "0, 0, 0")))

(event Input|MouseEvents|LeftMouseButton
  (params (Key :type Key%20Structure))
  (bind _returnvalue (Pawn|GetControlRotation :!class /Script/Engine.Pawn))
  (:Pressed
    (Game|SpawnActorfromClass "/Game/BluePrints/FlamingChair.FlamingChair_C" (Math|Transform|MakeTransform (+ (+ (Transformation|GetActorLocation) (stale _newparam1)) (* (Math|Vector|GetForwardVector _returnvalue) 1e+02)) _returnvalue) "Undefined" 0 0)))

(event Input|MouseEvents|RightMouseButton
  (params (Key :type Key%20Structure))
  (:Pressed
    (Utilities|FlowControl|Gate true) ; enters at Open
  )
  (:Released
    (Utilities|FlowControl|Gate true) ; enters at Close
  ))

(event Input|MouseEvents|RightMouseButton
  (params (Key :type Key%20Structure))
  (:Released
    (Transformation|SetActorRotation (Pawn|GetControlRotation :!class /Script/Engine.Pawn))))

(fn ConstructionScript)

(fn CameraZoom
  (params (Axis%20Value :type Float%20%28single-precision%29))
  (Variables|/Script/Engine.SpringArmComponent|SetTargetArmLength (Variables|Default|GetSpringArm) (Math|Float|Clamp(Float) (+ (Variables|/Script/Engine.SpringArmComponent|GetTargetArmLength (Variables|Default|GetSpringArm)) (* Axis%20Value 5e+01)) 1.5e+02 8e+02)))

(fn CameraRotation
  (bind _springarm (Variables|Default|GetSpringArm))
  (bind _returnvalue (Transformation|GetSocketTransform _springarm "None" "RTS_World"))
  (bind _rotation (Math|Transform|BreakTransform _returnvalue))
  (bind (_roll _pitch _yaw) (Math|Rotator|BreakRotator _rotation))
  (Transformation|SetRelativeRotation _springarm (Math|Rotator|MakeRotator 0.0 (+ _pitch (* (Class|Actor|GetInputAxisKeyValue) 2.0)) (+ _yaw (* (Class|Actor|GetInputAxisKeyValue) 2.0))) false false))

(fn FireDirection
  (bind _springarm (Variables|Default|GetSpringArm))
  (bind _returnvalue (Transformation|GetSocketTransform _springarm "None" "RTS_World"))
  (bind _rotation (Math|Transform|BreakTransform _returnvalue))
  (bind (_roll _pitch _yaw) (Math|Rotator|BreakRotator _rotation))
  (return (Math|Rotator|MakeRotator 0.0 (+ _pitch (* (Class|Actor|GetInputAxisKeyValue) 2.0)) (+ _yaw (* (Class|Actor|GetInputAxisKeyValue) 2.0)))))