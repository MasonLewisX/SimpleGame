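; Thrown chair projectile that turns mass and a randomized launch speed into a physics impact, with debug prints.
; On movement activation it rolls for a critical multiplier, then line-traces and pushes the hit component with an impulse scaled by damage, applying no actual damage.
; When the projectile stops, rotation halts and physics simulation starts.
; The camera view-point lookup, hit validity checks, fire effect and burning sound are all disconnected.
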(event `self.ProjectileMovement.OnComponentActivated`
  (params (Component :type "ActorComponent Object Reference") (bReset :type Boolean))
  (bind _returnvalue (`KismetMathLibrary.RandomFloatInRange` 100.0 300.0))
  (bind _starttrace (`self.StartTrace`))
  (bind _starttrace_2 (`self.StartTrace`))
  (bind _asprojectile_movement_component (cast `ProjectileMovementComponent` Component))
  (bind _output_get (set `ProjectileMovementComponent.InitialSpeed` _returnvalue _asprojectile_movement_component))
  (`KismetSystemLibrary.PrintString` (`KismetStringLibrary.Conv_DoubleToString` _returnvalue) true true (struct :`R` 0.156027 :`G` 0.157986 :`B` 0.153019 :`A` 1.0))
  (`KismetSystemLibrary.PrintString` "던지는 속도" true true (struct :`R` 0.156027 :`G` 0.157986 :`B` 0.153019 :`A` 1.0))
  (bind _output_get_2 (set `self.ChairBaseDamage` (* (`PrimitiveComponent.GetMass` (`self.Chair`)) _output_get)))
  (if (<= (`KismetMathLibrary.RandomFloatInRange` 0.0 100.0) (`self.CriticalHitProbability`))
    (bind _output_get_3 (set `self.Damage To Deal` (* _output_get_2 1.8)))
    (bind (_newparam _newparam1) (`self.GetPlayerViewPoint`))
    ;[1 1 1] CalculateAdjustedDirection
    (bind _output_get_4 (set `self.StartTrace` _newparam))
    (bind _output_get_5 (set `self.ShootDir` (`KismetMathLibrary.Conv_RotatorToVector` _newparam1)))
    ;[1 1 1] TraceShot
    (bind _outhit (`KismetSystemLibrary.LineTraceSingle` (+ (* _output_get_5 (`KismetMathLibrary.Dot_VectorVector` (- (`self.K2_GetActorLocation`) _output_get_4) _output_get_5)) _starttrace_2) (+ _starttrace_2 (* _output_get_5 (`self.WeaponRange`))) "TraceTypeQuery1"))
    (bind (_bblockinghit _binitialoverlap _time _distance _location _impactpoint _normal _impactnormal _physmat _hitactor _hitcomponent) (`GameplayStatics.BreakHitResult` _outhit))
    (bind _returnvalue_2 (+ _output_get_3 (stale _output_get_6)))
    ;[1 1 1] Deal With Impact
    (`PrimitiveComponent.AddImpulseAtLocation` _hitcomponent (* (`self.ShootDir`) _returnvalue_2) _location "None")
    (`KismetSystemLibrary.PrintString` (`KismetStringLibrary.Conv_DoubleToString` _returnvalue_2) true true (struct :`R` 1.0 :`B` 0.019054 :`A` 1.0))
    (`KismetSystemLibrary.PrintString` "치명타!!" true true (struct :`R` 1.0 :`B` 0.019054 :`A` 1.0))
    (else
      (bind _output_get_6 (set `self.Damage To Deal` _output_get_2))
      (bind (_newparam_2 _newparam1_2) (`self.GetPlayerViewPoint`))
      ;[1 1 1] CalculateAdjustedDirection
      (bind _output_get_7 (set `self.StartTrace` _newparam_2))
      (bind _output_get_8 (set `self.ShootDir` (`KismetMathLibrary.Conv_RotatorToVector` _newparam1_2)))
      ;[1 1 1] TraceShot
      (bind _outhit_2 (`KismetSystemLibrary.LineTraceSingle` (+ (* _output_get_8 (`KismetMathLibrary.Dot_VectorVector` (- (`self.K2_GetActorLocation`) _output_get_7) _output_get_8)) _starttrace) (+ _starttrace (* _output_get_8 (`self.WeaponRange`))) "TraceTypeQuery1"))
      (bind (_bblockinghit_2 _binitialoverlap_2 _time_2 _distance_2 _location_2 _impactpoint_2 _normal_2 _impactnormal_2 _physmat_2 _hitactor_2 _hitcomponent_2) (`GameplayStatics.BreakHitResult` _outhit_2))
      ;[1 1 1] Deal With Impact
      (`PrimitiveComponent.AddImpulseAtLocation` _hitcomponent_2 (* (`self.ShootDir`) _returnvalue_2) _location_2 "None")
      (`KismetSystemLibrary.PrintString` (`KismetStringLibrary.Conv_DoubleToString` _returnvalue_2))
      (`KismetSystemLibrary.PrintString` "데미지"))))

(event `self.ReceiveBeginPlay`)

(event `self.ProjectileMovement.OnProjectileStop`
  (params (ImpactResult :type "HitResult Structure (by ref)"))
  (set `RotatingMovementComponent.RotationRate` (struct) (`self.RotatingMovement`))
  (`PrimitiveComponent.SetSimulatePhysics` (`self.Collision`) true))

(fn `GetPlayerViewPoint`
  (returns (NewParam :type "Vector Structure") (NewParam1 :type "Rotator Structure"))
  (locals (MyPlayerController :type "PlayerController Object Reference")))

(fn `UserConstructionScript`)