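; AI controller for the Shinbi enemy, driving it through a behavior tree and blackboard.
; On possess it caches the Shinbi pawn and runs the tree; BeginPlay also sets the player key and runs it.
; AI Perception updates CanSeePlayer for ThirdPersonCharacter targets, saving the player's location and flagging RecentlySighted when sight is lost.
; Walk, Run, normal attack and dash attack events forward to the possessed pawn.
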(event `self.ReceiveBeginPlay`
  (bind _blackboardcomponent (`self.UseBlackboard` "/Game/BluePrints/AI_Shinbi/EnemyBlackboard_Shinbi.EnemyBlackboard_Shinbi"))
  (`BlackboardComponent.SetValueAsObject` _blackboardcomponent (`self.PlayerKey`) (`GameplayStatics.GetPlayerCharacter` 0))
  (`self.RunBehaviorTree` "/Game/BluePrints/AI_Shinbi/EnemyBehaviorTree_Shinbi.EnemyBehaviorTree_Shinbi"))

(event `self.AIPerception.OnTargetPerceptionUpdated`
  (params (Actor :type "Actor Object Reference") (Stimulus :type "AIStimulus Structure"))
  (bind (_age _expirationage _strength _stimuluslocation _receiverlocation _tag _bsuccessfullysensed) (break `AIStimulus` Stimulus))
  (bind _returnvalue (`AIBlueprintHelperLibrary.GetBlackboard` null))
  ;[1 1 1] 플레이어 감지 후 CanSeePlayer bool value true로 지정. 그 후 BehaviorTree 실행 순서에 의해 플레이어쪽으로 이동.
  (cast `/Game/ThirdPersonCPP/Blueprints/ThirdPersonCharacter` Actor)
  (`BlackboardComponent.SetValueAsBool` _returnvalue "CanSeePlayer" _bsuccessfullysensed)
  (if (not _bsuccessfullysensed)
    (`BlackboardComponent.SetValueAsVector` _returnvalue "PlayerLocation" (`self.K2_GetActorLocation` (`GameplayStatics.GetPlayerCharacter` 0)))
    (`BlackboardComponent.SetValueAsBool` _returnvalue "RecentlySighted" true)))

(event `Walk`
  ;[1 1 1] 필요없는 부분. 뭘 하던 없어도 됨.
  (`/Game/BluePrints/AI_Shinbi/ShinbiPlayerCharacter_AI.Walk` (`self.AIShinbi`)))

(event `Run`
  ;[1 1 1] 필요없는 부분. 뭘 하던 없어도 됨.
  (`/Game/BluePrints/AI_Shinbi/ShinbiPlayerCharacter_AI.Run` (`self.AIShinbi`)))

(event `self.OnPossess`
  (params (PossessedPawn :type "Pawn Object Reference"))
  (bind _asshinbi_player_character_ai (cast `/Game/BluePrints/AI_Shinbi/ShinbiPlayerCharacter_AI` PossessedPawn))
  (set `self.AIShinbi` _asshinbi_player_character_ai)
  (`self.RunBehaviorTree` "/Game/BluePrints/AI_Shinbi/EnemyBehaviorTree_Shinbi.EnemyBehaviorTree_Shinbi"))

(event `Attack_Normal`
  (`/Game/BluePrints/AI_Shinbi/ShinbiPlayerCharacter_AI.Attack_Normal` (`self.AIShinbi`)))

(event `Attack_Dash`
  (`/Game/BluePrints/AI_Shinbi/ShinbiPlayerCharacter_AI.Attack_Dash` (`self.AIShinbi`)))

(fn `UserConstructionScript`)